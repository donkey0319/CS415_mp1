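; BP_Ghost is an enemy actor that damages the player on contact and awards score when shot.
; A hit on its SK_Ghost component either takes one health from BP_Player or, for a BP_Projectile, adds one to the player's score, destroying the ghost in both cases.
; Each tick it also destroys itself once the player's health equals zero or the player's X location exceeds its own.
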(event OnComponentHit(SK_Ghost)
  (params (HitComponent :type Primitive%20Component%20Object%20Reference) (OtherActor :type Actor%20Object%20Reference) (OtherComp :type Primitive%20Component%20Object%20Reference) (NormalImpulse :type Vector :default "0, 0, 0") (Hit :type Hit%20Result%20Structure%20%28by%20ref%29))
  (Utilities|FlowControl|Sequence
    (:then_0
      (bind _asbp_player (Utilities|Casting|CastToBP_Player OtherActor))
      (Variables|/Game/InfiniteMatrix/Blueprints/BP_Player.BP_Player_C|SetHealth _asbp_player (- (Variables|/Game/InfiniteMatrix/Blueprints/BP_Player.BP_Player_C|GetHealth _asbp_player) 1.0))
      (Actor|DestroyActor))
    (:then_1
      (Utilities|Casting|CastToBP_Projectile OtherActor)
      (Actor|DestroyActor)
      (bind _asbp_player_2 (Utilities|Casting|CastToBP_Player (Game|Player|GetPlayerPawn 0)))
      (Variables|/Game/InfiniteMatrix/Blueprints/BP_Player.BP_Player_C|SetScore _asbp_player_2 (+ (Variables|/Game/InfiniteMatrix/Blueprints/BP_Player.BP_Player_C|GetScore _asbp_player_2) 1)))))

(event EventBeginPlay)

(event Collision|EventActorBeginOverlap
  (params (OtherActor :type Actor%20Object%20Reference)))

(event EventTick
  (params (DeltaSeconds :type Float%20%28single-precision%29))
  (bind _returnvalue (Game|Player|GetPlayerPawn 0))
  (Utilities|FlowControl|Sequence
    (:then_0
      (bind _asbp_player (Utilities|Casting|CastToBP_Player _returnvalue))
      (if (== (Variables|/Game/InfiniteMatrix/Blueprints/BP_Player.BP_Player_C|GetHealth _asbp_player) 0.0)
        (Actor|DestroyActor :!label _label)))
    (:then_1
      (if (> (.x (.location (Transformation|GetActorTransform _returnvalue))) (.x (.location (Transformation|GetActorTransform))))
        (goto _label)))))

(fn ConstructionScript)